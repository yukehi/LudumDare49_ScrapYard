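; CubeHandler is a Blueprint that controls a referenced cube, CurrentCube, and releases it on player input.
; BeginPlay stores the cube's starting location, and the ReleaseCubeKey action calls ReleaseCube on the cube.
; An IdleMoveCube function nudges the cube upward and prints its offset from the start, but nothing here calls it.
; Tick is empty, and the EnableInput call is left unconnected.
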(event EventBeginPlay
  (Variables|Default|SetInitalPosition (Transformation|GetActorLocation (Variables|Default|GetCurrentCube))))

(event Collision|EventActorBeginOverlap
  (params (OtherActor :type Actor%20Object%20Reference)))

(event EventTick
  (params (DeltaSeconds :type Float%20%28single-precision%29)))

(event Input|ActionEvents|InputActionReleaseCubeKey
  (params (Key :type Key%20Structure :default "None"))
  (:Pressed
    (Default|ReleaseCube (Variables|Default|GetCurrentCube))))

(fn ConstructionScript)

(fn IdleMoveCube
  (bind _currentcube (Variables|Default|GetCurrentCube))
  (Transformation|AddWorldOffset (Variables|/Game/Blueprints/Game_Cube.Game_Cube_C|GetCube _currentcube) "0,0.000000,1.000000" false false)
  (Development|PrintString (Utilities|String|ToString(Text) (Utilities|Text|ToText(String) (- (Variables|Default|GetInitalPosition) (Transformation|GetActorLocation _currentcube))))))